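; BP_Checkpoint is a lap trigger that starts the race and counts laps when its Box is overlapped.
; The first overlap starts a lap and the race through BP_RaceManager; later ones also increment and refresh BP_LevelOneGM's lap count, without filtering the overlapping actor.
; BeginPlay caches references through chained casts, casting the player pawn to both BP_PlayerCar and BP_AICar before reaching the game mode, so a failed cast leaves it unset.
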(event `self.Box.OnComponentBeginOverlap`
  (params (OverlappedComponent :type "PrimitiveComponent Object Reference") (OtherActor :type "Actor Object Reference") (OtherComp :type "PrimitiveComponent Object Reference") (OtherBodyIndex :type Integer) (bFromSweep :type Boolean) (SweepResult :type "HitResult Structure (by ref)"))
  (bind _as_bp_level_one_gm (`self.As BP Level One GM`))
  (bind _as_bp_race_manager (`self.As BP Race Manager`))
  ;[1 1 1] Component Overlap
  (if (`self.isRaceStarted?`)
    (`/Engine/EditorBlueprintResources/StandardMacros.IncrementInt` (`/Game/Blueprints/BP_LevelOneGM.LapsCompleted` _as_bp_level_one_gm)
      (:`  `
        (`/Game/Blueprints/BP_RaceManager.StartLap` _as_bp_race_manager)
        (`/Game/Blueprints/BP_LevelOneGM.UpdateLaps` _as_bp_level_one_gm)))
    (else
      (`/Game/Blueprints/BP_RaceManager.StartLap` _as_bp_race_manager)
      (`/Engine/EditorBlueprintResources/StandardMacros.DoOnce` false
        (:`Completed`
          (`/Game/Blueprints/BP_RaceManager.StartRace` _as_bp_race_manager)
          (set `self.isRaceStarted?` true))))))

(event `self.ReceiveBeginPlay`
  ;[1 1 1] Begin Play
  (bind _returnvalue (`GameplayStatics.GetActorOfClass` "/Game/Blueprints/BP_RaceManager.BP_RaceManager_C"))
  (bind _asbp_race_manager (cast `/Game/Blueprints/BP_RaceManager` _returnvalue))
  (set `self.As BP Race Manager` _asbp_race_manager)
  (bind _asbp_player_car (cast `/Game/Blueprints/BP_PlayerCar` (`GameplayStatics.GetPlayerPawn` 0)))
  (set `self.As BP Player Car` _asbp_player_car)
  (bind _asbp_aicar (cast `/Game/Blueprints/BP_AICar` (`GameplayStatics.GetPlayerPawn` 0)))
  (set `self.As BP AICar` _asbp_aicar)
  (bind _asbp_level_one_gm (cast `/Game/Blueprints/BP_LevelOneGM` (`GameplayStatics.GetGameMode`)))
  (set `self.As BP Level One GM` _asbp_level_one_gm))

(event `self.ReceiveActorBeginOverlap`
  (params (OtherActor :type "Actor Object Reference")))

(fn `UserConstructionScript`)