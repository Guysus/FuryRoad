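; BP_Starting_Point is the race start/finish trigger that starts the race and counts the player's laps.
; BeginPlay caches BP_RaceManager and casts the player pawn to both car classes.
; The first player overlap with PlayerCollision starts a lap and, through DoOnce, the race; later overlaps increment LapsCompleted, start a lap and update laps.
; The AICollision overlap is empty, and AI lap logic sits in disconnected nodes.
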(event `self.PlayerCollision.OnComponentBeginOverlap`
  (params (OverlappedComponent :type "PrimitiveComponent Object Reference") (OtherActor :type "Actor Object Reference") (OtherComp :type "PrimitiveComponent Object Reference") (OtherBodyIndex :type Integer) (bFromSweep :type Boolean) (SweepResult :type "HitResult Structure (by ref)"))
  (bind _as_bp_race_manager (`self.As BP Race Manager`))
  (bind _as_bp_race_manager_2 (`self.As BP Race Manager`))
  ;[1 1 1] Component Overlap
  (if (== (`GameplayStatics.GetPlayerPawn` 0) OtherActor)
    (if (`self.isRaceStarted?`)
      (bind _result (`/Engine/EditorBlueprintResources/StandardMacros.IncrementInt` (`/Game/Blueprints/BP_RaceManager.LapsCompleted` _as_bp_race_manager_2))
        (:`  `
          (set `/Game/Blueprints/BP_RaceManager.LapsCompleted` _result _as_bp_race_manager_2)
          (`/Game/Blueprints/BP_RaceManager.StartLap` _as_bp_race_manager_2)
          (`/Game/Blueprints/BP_RaceManager.UpdateLaps` _as_bp_race_manager_2)))
      (else
        (`/Game/Blueprints/BP_RaceManager.StartLap` _as_bp_race_manager)
        (`/Engine/EditorBlueprintResources/StandardMacros.DoOnce` false
          (:`Completed`
            (`/Game/Blueprints/BP_RaceManager.StartRace` _as_bp_race_manager)
            (set `self.isRaceStarted?` true)))))))

(event `self.ReceiveBeginPlay`
  ;[1 1 1] Begin Play
  (bind _returnvalue (`GameplayStatics.GetActorOfClass` "/Game/Blueprints/BP_RaceManager.BP_RaceManager_C"))
  (bind _asbp_race_manager (cast `/Game/Blueprints/BP_RaceManager` _returnvalue))
  (set `self.As BP Race Manager` _asbp_race_manager)
  (bind _asbp_player_car (cast `/Game/Blueprints/BP_PlayerCar` (`GameplayStatics.GetPlayerPawn` 0)))
  (set `self.As BP Player Car` _asbp_player_car)
  (bind _asbp_aicar (cast `/Game/Blueprints/BP_AICar` (`GameplayStatics.GetPlayerPawn` 0)))
  (set `self.As BP AICar` _asbp_aicar))

(event `self.ReceiveActorBeginOverlap`
  (params (OtherActor :type "Actor Object Reference")))

(event `self.AICollision.OnComponentBeginOverlap`
  (params (OverlappedComponent :type "PrimitiveComponent Object Reference") (OtherActor :type "Actor Object Reference") (OtherComp :type "PrimitiveComponent Object Reference") (OtherBodyIndex :type Integer) (bFromSweep :type Boolean) (SweepResult :type "HitResult Structure (by ref)")))

(fn `UserConstructionScript`)