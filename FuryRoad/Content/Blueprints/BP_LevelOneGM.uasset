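; BP_LevelOneGM is the level-one race manager that tracks lap progress and flags when the race is complete.
; BeginPlay resets completed laps, sets a two-lap requirement and refreshes the LapsAsText value.
; The UpdateLaps event refreshes that text, then sets IsRaceCompleted and prints a message once the requirement is met; nothing here increments LapsCompleted.
; In the LapsAsText function, the node chain that formats completed and required laps is marked unused.
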(event `self.ReceiveBeginPlay`
  ;[1 1 1] Begin Play
  (bind _output_get (set `self.LapsRequired` 2))
  (bind _output_get_2 (set `self.LapsCompleted` 0))
  (set `self.Laps as Text` (`self.LapsAsText` _output_get_2 _output_get)))

(event `UpdateLaps`
  (bind _lapscompleted (`self.LapsCompleted`))
  (bind _lapsrequired (`self.LapsRequired`))
  ;[1 1 1] Update Laps
  (set `self.Laps as Text` (`self.LapsAsText` _lapscompleted _lapsrequired))
  (if (>= _lapscompleted _lapsrequired)
    (set `self.isRaceCompleted?` true)
    (`KismetSystemLibrary.PrintString` "Race Completed")))

(fn `UserConstructionScript`)