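; BP_Checkpoints is a race checkpoint actor that registers when the player's pawn passes through it.
; On BeginPlay it finds the BP_RaceManager in the level and caches a reference to it.
; When the player pawn begins overlapping the PlayerCollision component, it increments the manager's completed checkpoint count, calls UpdateCheckpoints on the manager and prints a message.
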(event `self.ReceiveBeginPlay`
  (bind _returnvalue (`GameplayStatics.GetActorOfClass` "/Game/Blueprints/BP_RaceManager.BP_RaceManager_C"))
  (bind _asbp_race_manager (cast `/Game/Blueprints/BP_RaceManager` _returnvalue))
  (set `self.As BP Race Manager` _asbp_race_manager))

(event `self.PlayerCollision.OnComponentBeginOverlap`
  (params (OverlappedComponent :type "PrimitiveComponent Object Reference") (OtherActor :type "Actor Object Reference") (OtherComp :type "PrimitiveComponent Object Reference") (OtherBodyIndex :type Integer) (bFromSweep :type Boolean) (SweepResult :type "HitResult Structure (by ref)"))
  (bind _as_bp_race_manager (`self.As BP Race Manager`))
  ;[1 1 1] Player Car Collision
  (if (== (`GameplayStatics.GetPlayerPawn` 0) OtherActor)
    (bind _result (`/Engine/EditorBlueprintResources/StandardMacros.IncrementInt` (`/Game/Blueprints/BP_RaceManager.CP Completed` _as_bp_race_manager))
      (:`  `
        (set `/Game/Blueprints/BP_RaceManager.CP Completed` _result _as_bp_race_manager)
        (`/Game/Blueprints/BP_RaceManager.UpdateCheckpoints` (`self.As BP Race Manager`))
        (`KismetSystemLibrary.PrintString` "Update Checkpoint")))))

(fn `UserConstructionScript`)