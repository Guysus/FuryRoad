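; BP_AICar is an AI-driven car that follows the spline of an ActivePath reference at a constant half throttle set on BeginPlay.
; Each tick, GetPath projects a look-ahead point along the tangent of the nearest spline point and snaps it back onto the spline.
; The yaw difference between the car's heading and that target is mapped to a clamped steering input for the vehicle movement component.
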(event `self.ReceiveBeginPlay`
  (`ChaosVehicleMovementComponent.SetThrottleInput` (`self.VehicleMovementComponent`) 0.5))

(event `self.ReceiveTick`
  (params (DeltaSeconds :type "Float (single-precision)"))
  (bind _returnvalue (`self.GetPath`))
  (`ChaosVehicleMovementComponent.SetSteeringInput` (`self.VehicleMovementComponent`) _returnvalue))

(fn `GetPath`
  (returns (ReturnValue :type "Float (double-precision)"))
  (bind (_returnvalue_roll _returnvalue_pitch _returnvalue_yaw) (`KismetMathLibrary.BreakRotator` (`KismetMathLibrary.NormalizedDeltaRotator` (`KismetMathLibrary.FindLookAtRotation` (`self.K2_GetActorLocation`) (`SplineComponent.FindLocationClosestToWorldLocation` (`/Game/Blueprints/BP_Path.Spline` (`self.ActivePath`)) (+ (* (`KismetMathLibrary.Normal` (`SplineComponent.FindTangentClosestToWorldLocation` (`/Game/Blueprints/BP_Path.Spline` (`self.ActivePath`)) (`self.K2_GetActorLocation`) "World")) 200.0) (`self.K2_GetActorLocation`)) "World")) (`self.K2_GetActorRotation`))))
  (return (`KismetMathLibrary.MapRangeClamped` _returnvalue_yaw -90.0 90.0 -1.0 1.0)))

(fn `UserConstructionScript`)