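; BP_RaceManager tracks checkpoint, lap and race progress, showing a lap times widget from BeginPlay.
; Externally triggered update events refresh text and compare counts against targets set in BeginPlay.
; Meeting the checkpoint target cycles the lap timer and zeroes the count; meeting the lap target stops the race timer, shows the race-over widget and cursor.
; Two Timelines serve as clocks, writing formatted time text on update.
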(event `UpdateCheckpoints`
  (bind _cp_completed (`self.CP Completed`))
  (bind _cp_required (`self.CP Required`))
  ;[1 1 1] Update Checkpoints
  (set `self.Checkpoints as Text` (`/Game/Blueprints/BP_Macro_Library.CheckpointsAsText` _cp_completed _cp_required))
  (if (>= _cp_completed _cp_required)
    (`KismetSystemLibrary.PrintString` "Checkpoint condition met")
    (`self.EndLap`)
    (`self.StartLap`)
    (set `self.CP Completed` 0)
    (`KismetSystemLibrary.PrintString` "Reset Checkpoints")))

(event `RaceOver`
  ;[1 1 1] Race Over
  (if (`self.isRaceCompleted?`)
    (bind _returnvalue (`|CreateWidget` "/Game/Widgets/WB_Race_Over.WB_Race_Over_C"))
    (`UserWidget.AddToViewport` _returnvalue 0)))

(event `UpdateLaps`
  (bind _lapsrequired (`self.LapsRequired`))
  (bind _lapscompleted (`self.LapsCompleted`))
  ;[1 1 1] Update Laps
  (set `self.Laps as Text` (`/Game/Blueprints/BP_Macro_Library.LapsAsText` _lapscompleted _lapsrequired))
  (if (>= _lapscompleted _lapsrequired)
    (set `self.isRaceCompleted?` true)
    (`self.RaceOver`)
    (`self.EndRace`)
    (set `PlayerController.bShowMouseCursor` true (`GameplayStatics.GetPlayerController` 0))))

(event `StartLap`
  ;[1 1 1] Lap Timer
  (bind (_direction _time) (`Timeline|Timeline` :!label _label)
    (:`Update`
      (set `self.LapTimeAsText` (`/Game/Blueprints/BP_Macro_Library.TimeAsText` _time)))))

(event `EndLap`
  ;[1 1 1] Lap Timer
  (goto _label :!via `Stop`))

(event `StartRace`
  ;[1 1 1] Race Timer
  (bind (_direction _time) (`Timeline|Time` :!label _label_2)
    (:`Update`
      (set `self.RaceTime as Text` (`/Game/Blueprints/BP_Macro_Library.TimeAsText` _time)))))

(event `EndRace`
  ;[1 1 1] Race Timer
  (goto _label_2 :!via `Stop`))

(event `self.ReceiveBeginPlay`
  ;[1 1 1] Begin Play
  (bind _returnvalue (`|CreateWidget` "/Game/Widgets/WB_Lap_Times.WB_Lap_Times_C"))
  (bind _output_get (set `self.LapTimesWidget` _returnvalue))
  (`UserWidget.AddToViewport` _output_get 0)
  (bind _output_get_2 (set `self.LapsRequired` 2))
  (bind _output_get_3 (set `self.LapsCompleted` 0))
  (set `self.Laps as Text` (`/Game/Blueprints/BP_Macro_Library.LapsAsText` _output_get_3 _output_get_2))
  (bind _output_get_4 (set `self.CP Required` 28))
  (bind _output_get_5 (set `self.CP Completed` 0))
  (set `self.Checkpoints as Text` (`/Game/Blueprints/BP_Macro_Library.CheckpointsAsText` _output_get_5 _output_get_4)))

(fn `UserConstructionScript`)