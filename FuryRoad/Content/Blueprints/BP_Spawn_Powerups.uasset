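; BP_Spawn_Powerups is a pickup actor that restores health to the player car, despite its spawner-like name.
; Any overlap on its StaticMesh casts player pawn 0 to BP_PlayerCar, then destroys the pickup and plays a sound.
; It adds a fixed, unclamped amount to the car's CurrentHealth and calls UpdateHealth on the car.
; Game-instance health and random power-up selection nodes are unconnected leftovers.
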(event `self.ReceiveBeginPlay`)

(event `self.ReceiveActorBeginOverlap`
  (params (OtherActor :type "Actor Object Reference")))

(event `self.StaticMesh.OnComponentBeginOverlap`
  (params (OverlappedComponent :type "PrimitiveComponent Object Reference") (OtherActor :type "Actor Object Reference") (OtherComp :type "PrimitiveComponent Object Reference") (OtherBodyIndex :type Integer) (bFromSweep :type Boolean) (SweepResult :type "HitResult Structure (by ref)"))
  (bind _as_bp_player_car (`self.As BP Player Car`))
  (`KismetSystemLibrary.PrintString` "Hit Gas")
  (bind _asbp_player_car (cast `/Game/Blueprints/BP_PlayerCar` (`GameplayStatics.GetPlayerPawn` 0)))
  (bind _output_get (set `self.As BP Player Car` _asbp_player_car))
  (`self.K2_DestroyActor`)
  (`GameplayStatics.PlaySound2D` "/Game/SoundFX/drill.drill" 1.0 1.0 0.0 null null)
  (bind _output_get_2 (set `/Game/Blueprints/BP_PlayerCar.CurrentHealth` (+ (`/Game/Blueprints/BP_PlayerCar.CurrentHealth` _output_get) 20.0) _as_bp_player_car))
  (`/Game/Blueprints/BP_PlayerCar.UpdateHealth` _as_bp_player_car _output_get_2 (`/Game/Blueprints/BP_PlayerCar.MaxHealth` _as_bp_player_car)))

(fn `UserConstructionScript`)